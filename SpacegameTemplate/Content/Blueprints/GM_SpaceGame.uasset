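; GM_SpaceGame is the game mode that manages the main menu and player spawning.
; On BeginPlay it clears existing widgets, forces garbage collection, creates WG_MainMenu and shows it with UI-only input and a visible cursor.
; HideMenu restores game-only input and removes the menu.
; SpawnPlayer destroys every existing BP_Peter before spawning a fresh one.
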(event `Show Menu`
  (bind _returnvalue (`GameplayStatics.GetPlayerController` 0))
  (bind _wg_menu (`self.WG Menu`))
  (set `PlayerController.bShowMouseCursor` true _returnvalue)
  (`WidgetBlueprintLibrary.SetInputMode_UIOnlyEx` _returnvalue _wg_menu)
  (`UserWidget.AddToViewport` _wg_menu 0))

(event `self.ReceiveBeginPlay`
  (`WidgetLayoutLibrary.RemoveAllWidgets`)
  (`KismetSystemLibrary.CollectGarbage`)
  (bind _returnvalue (`|CreateWidget` "/Game/UI/WG_MainMenu.WG_MainMenu_C" (`GameplayStatics.GetPlayerController` 0)))
  (set `self.WG Menu` _returnvalue)
  (`self.Show Menu`))

(event `Spawn Player`
  (bind _outactors (`GameplayStatics.GetAllActorsOfClass` "/Game/Blueprints/BP_Peter.BP_Peter_C"))
  (for _array_element _outactors
    (`self.K2_DestroyActor` _array_element))
  (`|SpawnActorFromClass` "/Game/Blueprints/BP_Peter.BP_Peter_C" (`KismetMathLibrary.MakeTransform` (0.0 0.0 0.0)) "Undefined" "MultiplyWithRoot" null null))

(event `Hide Menu`
  (bind _returnvalue (`GameplayStatics.GetPlayerController` 0))
  (`WidgetBlueprintLibrary.SetInputMode_GameOnly` _returnvalue)
  (set `PlayerController.bShowMouseCursor` false _returnvalue)
  (`Widget.RemoveFromParent` (`self.WG Menu`)))

(fn `UserConstructionScript`)