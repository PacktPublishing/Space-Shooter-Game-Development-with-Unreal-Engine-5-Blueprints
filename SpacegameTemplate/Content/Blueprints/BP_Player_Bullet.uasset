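; Player projectile actor that flies in a given direction and damages enemies on contact.
; A BulletGo event sets the ProjectileMovement velocity from the direction and bullet speed.
; Mesh overlaps with ENEMY-tagged actors apply damage, then spawn an explosion and destroy the bullet.
; Overlaps with BASE-tagged actors only explode and destroy it, and other overlaps are ignored.
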(event `Bullet Go`
  (params (Direction :type "Vector Structure"))
  (set `MovementComponent.Velocity` (* Direction (`self.Bullet_Speed`)) (`self.ProjectileMovement`)))

(event `self.StaticMesh.OnComponentBeginOverlap`
  (params (OverlappedComponent :type "PrimitiveComponent Object Reference") (OtherActor :type "Actor Object Reference") (OtherComp :type "PrimitiveComponent Object Reference") (OtherBodyIndex :type Integer) (bFromSweep :type Boolean) (SweepResult :type "HitResult Structure (by ref)"))
  (if (`self.ActorHasTag` OtherActor "ENEMY")
    (`GameplayStatics.ApplyDamage` OtherActor (`self.Base Damage`))
    (`GameplayStatics.SpawnEmitterAtLocation` "/Game/Particles/P_Explosion.P_Explosion" (`self.K2_GetActorLocation`) :!label _label)
    (`self.K2_DestroyActor`)
    (elif (`self.ActorHasTag` OtherActor "BASE")
      (goto _label))))

(fn `UserConstructionScript`)