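; Player missile that chases an enemy target or flies along a launch vector and deals area damage on impact.
; A valid enemy target is chased by moving the actor each Tick; otherwise ProjectileMovement drives it and enables the Sphere seek trigger, which can switch on projectile homing.
; Sphere1 detects enemy or base contact, damages enemies inside DamageCol and destroys the missile.
; Destruction, from any cause, spawns an explosion emitter.
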(event `self.ReceiveTick`
  (params (DeltaSeconds :type "Float (single-precision)"))
  (if (`self.Homing`)
    (`/Engine/EditorBlueprintResources/StandardMacros.IsValid` (`self.Homing Target`)
      (:`Is Valid`
        (`self.K2_SetActorLocation` (`KismetMathLibrary.VInterpTo_Constant` (`self.K2_GetActorLocation`) (`self.K2_GetActorLocation` (`self.Homing Target`)) DeltaSeconds 50000.0)))
      (:`Is Not Valid`
        (set `self.Homing` false)
        (set `PrimitiveComponent.bGenerateOverlapEvents` true (`self.Sphere`))))))

(event `Launch Missile`
  (params (`Target Vector` :type "Vector Structure") (`Target actor` :type "Actor Object Reference"))
  (set `self.Target Vector` `Target Vector`)
  (bind _output_get (set `self.Homing Target` `Target actor`))
  (`/Engine/EditorBlueprintResources/StandardMacros.IsValid` _output_get
    (:`Is Valid`
      (if (`self.ActorHasTag` (`self.Homing Target`) "ENEMY")
        (set `self.Homing` true)
        (else
          (set `MovementComponent.Velocity` (* (`self.Target Vector`) 20000) (`self.ProjectileMovement`) :!label _label)
          (set `PrimitiveComponent.bGenerateOverlapEvents` true (`self.Sphere`)))))
    (:`Is Not Valid`
      (goto _label))))

(event `self.ReceiveBeginPlay`
  (add `self.OnDestroyed` (delegate `Missile Explode`)))

(event `Missile Explode` :!signature `self.OnDestroyed`
  (params (DestroyedActor :type "Actor Object Reference"))
  (`GameplayStatics.SpawnEmitterAtLocation` "/Game/Particles/P_Explosion.P_Explosion" (`self.K2_GetActorLocation`) (struct) (20.0 20.0 20.0)))

(event `self.Sphere.OnComponentBeginOverlap`
  (params (OverlappedComponent :type "PrimitiveComponent Object Reference") (OtherActor :type "Actor Object Reference") (OtherComp :type "PrimitiveComponent Object Reference") (OtherBodyIndex :type Integer) (bFromSweep :type Boolean) (SweepResult :type "HitResult Structure (by ref)"))
  (if (`self.ActorHasTag` OtherActor "Enemy")
    (`/Engine/EditorBlueprintResources/StandardMacros.DoOnce` (`self.Homing`)
      (:`Completed`
        (set `self.Homing Target` OtherActor)
        (`self.Set Homing`)))))

(event `self.Sphere1.OnComponentBeginOverlap`
  (params (OverlappedComponent :type "PrimitiveComponent Object Reference") (OtherActor :type "Actor Object Reference") (OtherComp :type "PrimitiveComponent Object Reference") (OtherBodyIndex :type Integer) (bFromSweep :type Boolean) (SweepResult :type "HitResult Structure (by ref)"))
  (if (or (`self.ActorHasTag` OtherActor "Enemy") (`self.ActorHasTag` OtherActor "BASE"))
    (`/Engine/EditorBlueprintResources/StandardMacros.DoOnce` false
      (:`Completed`
        (for _array_element (`PrimitiveComponent.GetOverlappingActors` (`self.Damage col`) null)
          (if (`self.ActorHasTag` _array_element "Enemy")
            (`GameplayStatics.ApplyDamage` _array_element 10.0)))
        (`self.K2_DestroyActor`)))))

(fn `Set Homing`
  (bind _projectilemovement (`self.ProjectileMovement`))
  (set `MovementComponent.Velocity` (0.0 0.0 0.0) _projectilemovement)
  (set `ProjectileMovementComponent.bIsHomingProjectile` true _projectilemovement)
  (set `ProjectileMovementComponent.HomingTargetComponent` (`self.GetComponentByClass` (`self.Homing Target`) "/Script/Engine.SceneComponent") _projectilemovement))

(fn `UserConstructionScript`)