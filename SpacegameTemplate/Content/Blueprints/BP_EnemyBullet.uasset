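; BP_EnemyBullet is an enemy projectile that damages the player on contact.
; A BulletGo event sets the projectile movement velocity from a given direction and bullet speed.
; When its mesh overlaps a PLAYER-tagged BP_Peter, it counts a hit only against the Body component, then applies damage, spawns an explosion effect and destroys itself.
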(event `self.StaticMesh.OnComponentBeginOverlap`
  (params (OverlappedComponent :type "PrimitiveComponent Object Reference") (OtherActor :type "Actor Object Reference") (OtherComp :type "PrimitiveComponent Object Reference") (OtherBodyIndex :type Integer) (bFromSweep :type Boolean) (SweepResult :type "HitResult Structure (by ref)"))
  (if (`self.ActorHasTag` OtherActor "PLAYER")
    (bind _asbp_peter (cast `/Game/Blueprints/BP_Peter` OtherActor))
    (if (== (`/Game/Blueprints/BP_Peter.Body` _asbp_peter) OtherComp)
      (`GameplayStatics.ApplyDamage` _asbp_peter 1.0)
      (`GameplayStatics.SpawnEmitterAtLocation` "/Game/Particles/P_Explosion.P_Explosion" (`self.K2_GetActorLocation`))
      (`self.K2_DestroyActor`))))

(event `Bullet Go`
  (params (Direction :type "Vector Structure"))
  (set `MovementComponent.Velocity` (* Direction (`self.Bullet_Speed`)) (`self.ProjectileMovement`)))

(fn `UserConstructionScript`)