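; Player spaceship pawn for a flying shooter, which also runs enemy spawning and score-based upgrades.
; Tick drives six-direction key movement, strafe banking and a camera line trace that aims lasers and missiles.
; Timers handle stamina-limited sprint, health regeneration while idle and randomly delayed Kamikaze and Shooter spawns around the ship, with destroy callbacks maintaining enemy counts.
; Score unlocks missiles and upgraded guns, the crosshair widget shows status, and death shows game-over.
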(event `self.ReceiveTick`
  (params (DeltaSeconds :type "Float (single-precision)"))
  ;[1 1 1] Tick
  (`|ExecutionSequence`
    (:`then_0`
      ;[1 1 1] Movement
      (`PawnMovementComponent.AddInputVector` (`self.FloatingPawnMovement`) (`self.Movement Math simple`) false))
    (:`then_1`
      ;[1 1 1] Rotate Ship When Strafe Math
      (`self.Rotate Ship When Strafe`))
    (:`then_2`
      (`self.Targeting`))))

(event `Start Spawn`
  ;[1 1 1] Spawn
  (`KismetSystemLibrary.K2_SetTimerDelegate` (delegate `Spawning Timer`) (`KismetMathLibrary.RandomFloatInRange` 1.0 5.0)))

(event `Spawning Timer`
  ;[1 1 1] Spawn
  (`|ExecutionSequence`
    (:`then_0`
      (`self.Start Spawn`))
    (:`then_1`
      (if (not (>= (`self.Spawn Counter`) (`self.Max Default Enemy`)))
        (bind _returnvalue (`|SpawnActorFromClass` "/Game/Blueprints/BP_Enemy_Kamikaze.BP_Enemy_Kamikaze_C" (`KismetMathLibrary.MakeTransform` (+ (`self.K2_GetActorLocation`) (* (`KismetMathLibrary.RandomUnitVector`) 30000)) (struct) (3.0 3.0 3.0)) "Undefined" "MultiplyWithRoot" self null))
        (add `self.OnDestroyed` _returnvalue (delegate `On Death OfLvl 1`))
        (set `self.Spawn Counter` (+ (`self.Spawn Counter`) 1))))
    (:`then_2`
      (if (> (`self.Score`) 8)
        (if (not (>= (`self.Lvl2 Spawn Counter`) (`self.Max Default Enemy`)))
          (bind _returnvalue_2 (`|SpawnActorFromClass` "/Game/Blueprints/BP_Shooter.BP_Shooter_C" (`KismetMathLibrary.MakeTransform` (+ (`self.K2_GetActorLocation`) (* (`KismetMathLibrary.RandomUnitVector`) 30000)) (struct) (3.0 3.0 3.0)) "Undefined" "MultiplyWithRoot" self null))
          (add `self.OnDestroyed` _returnvalue_2 (delegate `Death of lvl 2`))
          (set `self.Lvl2 Spawn Counter` (+ (`self.Lvl2 Spawn Counter`) 1)))))))

(event `On Death OfLvl 1` :!signature `self.OnDestroyed`
  (params (DestroyedActor :type "Actor Object Reference"))
  ;[1 1 1] Spawn
  (set `self.Spawn Counter` (- (`self.Spawn Counter`) 1))
  (`self.Start Spawn`))

(event `Death of lvl 2` :!signature `self.OnDestroyed`
  (params (DestroyedActor :type "Actor Object Reference"))
  ;[1 1 1] Spawn
  (set `self.Lvl2 Spawn Counter` (- (`self.Lvl2 Spawn Counter`) 1))
  (`self.Start Spawn`))

(event `Start Sprint`
  ;[1 1 1] Sprint Visuals
  (bind (_direction _newtrack_0) (`Timeline|TL Sprint` :!label _label)
    (:`Update`
      (`SceneComponent.SetWorldScale3D` (`self.ParticleSystem7`) (`KismetMathLibrary.VLerp` (0.25 0.5 0.5) (0.5 0.5 1.5) _newtrack_0))
      (`SceneComponent.SetWorldScale3D` (`self.ParticleSystem6`) (`KismetMathLibrary.VLerp` (0.25 0.5 0.5) (0.5 0.5 1.5) _newtrack_0))
      (`SceneComponent.SetWorldScale3D` (`self.ParticleSystem5`) (`KismetMathLibrary.VLerp` (0.25 0.5 0.5) (0.5 0.5 1.5) _newtrack_0))
      (`SceneComponent.SetWorldScale3D` (`self.ParticleSystem4`) (`KismetMathLibrary.VLerp` (0.25 0.5 0.5) (0.5 0.5 1.5) _newtrack_0))
      (`CameraComponent.SetFieldOfView` (`self.Camera`) (`KismetMathLibrary.Lerp` 90.0 110.0 _newtrack_0)))))

(event `Stamina_Regen`
  ;[1 1 1] Timer Stamina management
  (set `self.Stamina` (`KismetMathLibrary.FClamp` (select `bool` (`self.Is_Sprinting`) :`false` (+ (`self.Stamina`) 1.0) :`true` (- (`self.Stamina`) 1.0)) 0.0 (`self.Max Stamina`)))
  (`/Game/UI/WG_Crosshair.Set Stamina Percent` (`self.UI reference`) (/ (`self.Stamina`) (`self.Max Stamina`)))
  (`|ExecutionSequence`
    (:`then_0`
      (if (>= (`self.Stamina`) (`self.Max Stamina`))
        (`KismetSystemLibrary.K2_PauseTimerHandle` (`self.Stamina Timer handle`))))
    (:`then_1`
      (if (== (`self.Stamina`) 0.0)
        (`self.Stop Sprint`)))))

(event `Key|W`
  (params (Key :type "Key Structure"))
  ;[1 1 1] Movement Inputs
  (:`Pressed`
    (set `self.W Pressed` true))
  (:`Released`
    (set `self.W Pressed` false)))

(event `End Sprint`
  ;[1 1 1] Sprint Visuals
  (goto _label :!via `Reverse`))

(event `Key|SpaceBar`
  (params (Key :type "Key Structure"))
  ;[1 1 1] Movement Inputs
  (:`Pressed`
    (set `self.Space Pressed` true))
  (:`Released`
    (set `self.Space Pressed` false)))

(event `InputAxisKey|MouseX`
  (params (AxisValue :type "Float (single-precision)"))
  ;[1 1 1] Mouse X Y
  (bind _output_get (set `self.Mouse X` AxisValue))
  (`self.AddControllerYawInput` (* _output_get (`self.Sensitivity X`))))

(event `self.ReceiveBeginPlay`
  (bind _ui_reference (`self.UI reference`))
  ;[1 1 1] Begin Play / Possess Character/ Enable Inputs
  (`Controller.Possess` (`GameplayStatics.GetPlayerController` 0) self)
  ;[1 1 1] Store Default Values and references
  (`self.Set Default Values And References`)
  (`|ExecutionSequence`
    (:`then_0`
      ;[1 1 1] Create and add to vieport the UI
      (bind _returnvalue (`|CreateWidget` "/Game/UI/WG_Crosshair.WG_Crosshair_C" (`GameplayStatics.GetPlayerController` 0)))
      (set `self.UI reference` _returnvalue)
      (`/Game/UI/WG_Crosshair.Set Health Percent` _ui_reference 1.0)
      (`UserWidget.AddToViewport` _ui_reference 0))
    (:`then_1`
      ;[1 1 1] Timer Stamina management
      (bind _returnvalue_2 (`KismetSystemLibrary.K2_SetTimerDelegate` (delegate `Stamina_Regen`) 1.0 true))
      (set `self.Stamina Timer handle` _returnvalue_2))
    (:`then_2`
      ;[1 1 1] Shooting Timer
      (bind _returnvalue_3 (`KismetSystemLibrary.K2_SetTimerDelegate` (delegate `Fire Check`) (`self.Laser Cooldown_Timer`) true))
      (set `self.Main Gun Timer` _returnvalue_3)
      (`KismetSystemLibrary.K2_PauseTimerHandle` (`self.Main Gun Timer`)))
    (:`then_3`
      ;[1 1 1] Player Regen
      (`KismetSystemLibrary.K2_SetTimerDelegate` (delegate `Regen Timer`) 0.1 true))
    (:`then_4`
      (`KismetSystemLibrary.Delay` 3.0)
      (`self.Start Spawn`))))

(event `Key|LeftControl`
  (params (Key :type "Key Structure"))
  ;[1 1 1] Movement Inputs
  (:`Pressed`
    (set `self.Cntrl Pressed` true))
  (:`Released`
    (set `self.Cntrl Pressed` false)))

(event `Key|A`
  (params (Key :type "Key Structure"))
  ;[1 1 1] Movement Inputs
  (:`Pressed`
    (set `self.A pressed` true))
  (:`Released`
    (set `self.A pressed` false)))

(event `Key|D`
  (params (Key :type "Key Structure"))
  ;[1 1 1] Movement Inputs
  (:`Pressed`
    (set `self.D Pressed` true))
  (:`Released`
    (set `self.D Pressed` false)))

(event `Key|S`
  (params (Key :type "Key Structure"))
  ;[1 1 1] Movement Inputs
  (:`Pressed`
    (set `self.S Pressed` true))
  (:`Released`
    (set `self.S Pressed` false)))

(event `InputAxisKey|MouseY`
  (params (AxisValue :type "Float (single-precision)"))
  ;[1 1 1] Mouse X Y
  (bind _output_get (set `self.Mouse Y` AxisValue))
  (`self.AddControllerPitchInput` (* (* _output_get -1.0) (`self.Sensitivity Y`))))

(event `Fire Check`
  ;[1 1 1] Shooting Timer
  (if (`self.Is_Firing`)
    _))

(event `Key|RightMouseButton`
  (params (Key :type "Key Structure"))
  (bind _gun_1 (`self.Gun 1`))
  (bind (_target_direcion _target_actor) (`self.Targeting Crosshair Math` (`self.Gun 1`)))
  ;[1 1 1] Missile
  (:`Pressed`
    (if (`self.Has Missile`)
      (set `self.Has Missile` false)
      (`/Game/UI/WG_Crosshair.Missile in CD` (`self.UI reference`))
      (bind _returnvalue (`|SpawnActorFromClass` "/Game/Blueprints/BP_PlayerMissile.BP_PlayerMissile_C" (`KismetMathLibrary.MakeTransform` (`SceneComponent.K2_GetComponentLocation` _gun_1) (`SceneComponent.K2_GetComponentRotation` _gun_1)) "Undefined" "MultiplyWithRoot" null null))
      (`/Game/Blueprints/BP_PlayerMissile.Launch Missile` _returnvalue _target_direcion _target_actor)
      (`GameplayStatics.PlaySound2D` "/Game/Sounds/458669__jorgerosa__missile-launch.458669__jorgerosa__missile-launch" 2.0 1.0 0.0 null null)
      (`KismetSystemLibrary.Delay` 0.3)
      (set `self.Has Missile` true)
      (`/Game/UI/WG_Crosshair.Missile Not in CD` (`self.UI reference`)))))

(event `Key|LeftShift`
  (params (Key :type "Key Structure"))
  ;[1 1 1] Sprint
  (:`Pressed`
    (if (not (== (`self.Stamina`) 0.0))
      (set `FloatingPawnMovement.MaxSpeed` 2500.0 (`self.FloatingPawnMovement`))
      (set `self.Is_Sprinting` true)
      (`self.Start Sprint`)
      (`KismetSystemLibrary.K2_UnPauseTimerHandle` (`self.Stamina Timer handle`))))
  (:`Released`
    (`self.Stop Sprint`)))

(event `/Game/Blueprints/BI_Coms.UpdateVisuals`
  (params (Hp :type "Float (double-precision)") (Dead :type Boolean))
  ;[1 1 1] Ui Visuals-Death
  (if Dead
    (`self.Death`)
    (else
      (`/Game/UI/WG_Crosshair.Set Health Percent` (`self.UI reference`) (/ Hp (`/Game/Blueprints/BPC_Damagable.Max Health` (`self.BPC_Damagable`)))))))

(event `Regen Timer`
  ;[1 1 1] Player Regen
  (if (not (or (`self.Is_Firing`) (not (== (`self.GetVelocity`) (0.0 0.0 0.0)))))
    (`/Game/Blueprints/BPC_Damagable.Give Health` (`self.BPC_Damagable`) 0.1)))

(event `/Game/Blueprints/BI_Coms.Points Update`
  (params (Points :type Integer))
  ;[1 1 1] Update Score
  (set `self.Score` (+ (`self.Score`) Points))
  (`/Game/UI/WG_Crosshair.Update Score` (`self.UI reference`) (`self.Score`))
  (switch `string` (`KismetStringLibrary.Conv_IntToString` (`self.Score`))
    (:`5`
      (set `self.Has Missile` true)
      (`Widget.SetVisibility` (`/Game/UI/WG_Crosshair.Img_Missile` (`self.UI reference`)) "Visible")
      (`GameplayStatics.PlaySound2D` "/Game/Sounds/607409__colorscrimsontears__upgrade_Cue.607409__colorscrimsontears__upgrade_Cue" 1.0 1.0 0.0 null null))
    (:`10`
      (`/Engine/EditorBlueprintResources/StandardMacros.IncrementInt` (`self.Weapon Lvl`)
        (:`  `
          (set `self.Laser Cooldown_Timer` 0.15)
          (set `self.Max Default Enemy` 12)
          (`GameplayStatics.PlaySound2D` "/Game/Sounds/607409__colorscrimsontears__upgrade_Cue.607409__colorscrimsontears__upgrade_Cue" 1.0 1.0 0.0 null null))))))

(event `Fire Laser`
  ;[1 1 1] Fire Laser
  (`/Engine/EditorBlueprintResources/StandardMacros.DoOnce` false :!label _label_2
    (:`Completed`
      (`|ExecutionSequence`
        (:`then_0`
          (`GameplayStatics.PlaySound2D` "/Game/Sounds/617034__d4xx__laser-shot_Cue.617034__d4xx__laser-shot_Cue" 1.0 1.0 0.0 null null)
          (`KismetSystemLibrary.Delay` (`self.Laser Cooldown_Timer`))
          (`self.Reset Fire Laser`)
          (if (`self.Is_Firing`)
            (`self.Fire Laser`)))
        (:`then_1`
          (switch `int` (`self.Weapon Lvl`)
            (:`0`
              (`self.Shoot Bullet` (`self.Gun 1`)))
            (:`1`
              (bind _isa (`/Engine/EditorBlueprintResources/StandardMacros.FlipFlop`)
                (:`A`
                  _)
                (:`B`
                  _))
              (`self.Shoot Bullet` (select `bool` _isa :`false` (`self.Gun 2`) :`true` (`self.Gun 3`))))))))))

(event `Reset Fire Laser`
  ;[1 1 1] Fire Laser
  (goto _label_2 :!via `Reset`))

(event `Key|LeftMouseButton`
  (params (Key :type "Key Structure"))
  (bind _main_gun_timer (`self.Main Gun Timer`))
  ;[1 1 1] Main_Gun_Shooting
  (:`Pressed`
    (set `self.Is_Firing` true)
    (`KismetSystemLibrary.K2_UnPauseTimerHandle` _main_gun_timer)
    (`self.Fire Laser`))
  (:`Released`
    (set `self.Is_Firing` false)
    (`KismetSystemLibrary.K2_PauseTimerHandle` _main_gun_timer)))

(event `ddf`)

(fn `Death`
  (`self.DisableInput` (`GameplayStatics.GetPlayerController` 0))
  (`self.SetActorHiddenInGame` true)
  (`GameplayStatics.SpawnEmitterAtLocation` "/Game/Particles/P_Explosion.P_Explosion" (`self.K2_GetActorLocation`) (struct) (8.0 8.0 8.0))
  (bind _returnvalue (`|CreateWidget` "/Game/UI/WG_Gameover.WG_Gameover_C" (`GameplayStatics.GetPlayerController` 0)))
  (`UserWidget.AddToViewport` _returnvalue 0)
  (`self.K2_DestroyActor`))

(fn `Movement Math`
  (returns (ReturnValue :type "Vector Structure"))
  (bind _returnvalue (`self.GetActorForwardVector`))
  (bind _returnvalue_2 (`self.GetActorRightVector`))
  (bind _returnvalue_3 (`|GetInputActionValue`))
  (bind _x (`KismetMathLibrary.BreakVector2D` (`|GetInputActionValue`)))
  (bind _x_2 (`KismetMathLibrary.BreakVector2D` (`|GetInputActionValue`)))
  (bind (_x_3 _y) (`KismetMathLibrary.BreakVector2D` (`|GetInputActionValue`)))
  (bind (_x_4 _y_2) (`KismetMathLibrary.BreakVector2D` (`|GetInputActionValue`)))
  (set `self.Dirrection_FB` (`KismetMathLibrary.SelectVector` (0.0 0.0 0.0) (`KismetMathLibrary.SelectVector` (* _returnvalue -1) _returnvalue (< _y 0.0)) (or (and (== _y -1.0) (== _y_2 1.0)) (and (== _y 0.0) (== _y_2 0.0)))))
  (set `self.Dirrection_LR` (`KismetMathLibrary.SelectVector` (0.0 0.0 0.0) (`KismetMathLibrary.SelectVector` (* _returnvalue_2 -1) _returnvalue_2 (< _x_2 0.0)) (or (and (== _x_2 -1.0) (== _x 1.0)) (and (== _x_2 0.0) (== _x 0.0)))))
  (set `self.Dirrection_UpDown` (`KismetMathLibrary.SelectVector` (0.0 0.0 0.0) (select `bool` (> _returnvalue_3 0.0) :`false` (* (`self.GetActorUpVector`) -1) :`true` (`self.GetActorUpVector`)) (== _returnvalue_3 0.0)))
  (return (+ (`self.Dirrection_FB`) (`self.Dirrection_LR`) (`self.Dirrection_UpDown`))))

(fn `Movement Math simple`
  (returns (ReturnValue :type "Vector Structure"))
  (bind _returnvalue (`self.GetActorForwardVector`))
  (bind _returnvalue_2 (`self.GetActorRightVector`))
  (bind _d_pressed (`self.D Pressed`))
  (bind _cntrl_pressed (`self.Cntrl Pressed`))
  (bind _a_pressed (`self.A pressed`))
  (bind _space_pressed (`self.Space Pressed`))
  (set `self.Dirrection_FB` (`KismetMathLibrary.SelectVector` (0.0 0.0 0.0) (`KismetMathLibrary.SelectVector` (* _returnvalue -1) _returnvalue (`self.S Pressed`)) (or (and (`self.W Pressed`) (`self.S Pressed`)) (and (not (`self.W Pressed`)) (not (`self.S Pressed`))))))
  (set `self.Dirrection_LR` (`KismetMathLibrary.SelectVector` (0.0 0.0 0.0) (`KismetMathLibrary.SelectVector` (* _returnvalue_2 -1) _returnvalue_2 (`self.A pressed`)) (or (and _a_pressed _d_pressed) (and (not _a_pressed) (not _d_pressed)))))
  (set `self.Dirrection_UpDown` (`KismetMathLibrary.SelectVector` (0.0 0.0 0.0) (select `bool` (`self.Space Pressed`) :`false` (* (`self.GetActorUpVector`) -1) :`true` (`self.GetActorUpVector`)) (or (and _space_pressed _cntrl_pressed) (and (not _space_pressed) (not _cntrl_pressed)))))
  (return (+ (`self.Dirrection_FB`) (`self.Dirrection_LR`) (`self.Dirrection_UpDown`))))

(fn `Rotate Ship When Strafe`
  (bind _a_pressed (`self.A pressed`))
  (bind _d_pressed (`self.D Pressed`))
  (bind _body_original_relative_rotation (`self.Body Original Relative Rotation`))
  (if (or (and _a_pressed _d_pressed) (and (not _a_pressed) (not _d_pressed)))
    (`SceneComponent.K2_SetRelativeRotation` (`self.Body`) (`KismetMathLibrary.RInterpTo` (`SceneComponent.RelativeRotation` (`self.Body`)) (`self.Body Original Relative Rotation`) (`GameplayStatics.GetWorldDeltaSeconds`) 1.0) false false)
    (else
      (`SceneComponent.K2_SetRelativeRotation` (`self.Body`) (`KismetMathLibrary.RInterpTo` (`SceneComponent.RelativeRotation` (`self.Body`)) (`KismetMathLibrary.ComposeRotators` (`self.Body Original Relative Rotation`) (`KismetMathLibrary.SelectRotator` (`KismetMathLibrary.ComposeRotators` _body_original_relative_rotation (struct :`Roll` -15.0)) (`KismetMathLibrary.ComposeRotators` _body_original_relative_rotation (struct :`Roll` 15.0)) (`self.A pressed`))) (`GameplayStatics.GetWorldDeltaSeconds`) 1.0) false false))))

(fn `Set Default Values And References`
  (set `self.Body Original Relative Rotation` (`SceneComponent.RelativeRotation` (`self.Body`))))

(fn `Shoot Bullet`
  (params (InputPin :type "SceneComponent Object Reference"))
  (bind _returnvalue (`|SpawnActorFromClass` "/Game/Blueprints/BP_Player_Bullet.BP_Player_Bullet_C" (`SceneComponent.K2_GetComponentToWorld` InputPin) "Undefined" "MultiplyWithRoot" self self))
  (`/Game/Blueprints/BP_Player_Bullet.Bullet Go` _returnvalue (`self.Targeting Crosshair Math` InputPin)))

(fn `Stop Sprint`
  (set `self.Is_Sprinting` false)
  (set `FloatingPawnMovement.MaxSpeed` 1500.0 (`self.FloatingPawnMovement`))
  (`self.End Sprint`))

(fn `Targeting`
  (locals (`Target direction` :type "Vector Structure"))
  (bind _camera (`self.Camera`))
  (bind _ui_reference (`self.UI reference`))
  (set `self.Target Directionn` (+ (`SceneComponent.K2_GetComponentLocation` _camera) (* (`SceneComponent.GetForwardVector` _camera) 50000)))
  (bind (_outhit _returnvalue) (`KismetSystemLibrary.LineTraceSingleForObjects` :`Start` (`SceneComponent.K2_GetComponentLocation` (`self.Camera`)) :`End` (`self.Target Directionn`) :`ObjectTypes` (`self.Main Gun Trace Object Types`) :`DrawTime` 55.0))
  (if _returnvalue
    (`/Game/UI/WG_Crosshair.Crosshair has Target` _ui_reference)
    (bind (_bblockinghit _binitialoverlap _time _distance _location _impactpoint _normal _impactnormal _physmat _hitactor) (`GameplayStatics.BreakHitResult` _outhit))
    (set `self.Target Directionn` _location)
    (set `self.Target Actor Ref` _hitactor)
    (else
      (`/Game/UI/WG_Crosshair.Crosshair No target` _ui_reference)
      (set `self.Target Actor Ref` null))))

(fn `Targeting Crosshair Math`
  (params (`Shooting Point` :type "SceneComponent Object Reference"))
  (returns (`Target Direcion` :type "Vector Structure") (`Target Actor` :type "Actor Object Reference"))
  (bind _returnvalue (`SceneComponent.K2_GetComponentLocation` (`local.Shooting Point`)))
  (set `self.Target Directionn` (`KismetMathLibrary.Normal` (- (+ _returnvalue (- (`self.Target Directionn`) _returnvalue)) (`SceneComponent.K2_GetComponentLocation` (`local.Shooting Point`)))))
  (return (`self.Target Directionn`) (`self.Target Actor Ref`)))

(fn `Upgrade`
  (params (`WG Text` :type Text))
  (switch `string` (`KismetTextLibrary.Conv_TextToString` `WG Text`)))

(fn `UserConstructionScript`)