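; BPC_Damagable is an actor component that adds health to its owning actor.
; On BeginPlay it binds to the owner's OnTakeAnyDamage and passes incoming damage to RemoveHealth, while GiveHealth provides the healing counterpart.
; Both functions clamp health between zero and MaxHealth, then send the owner an UpdateVisuals interface message with the new value and a death flag, leaving the visual response to the owner.
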(event `self.ReceiveBeginPlay`
  (add `Actor.OnTakeAnyDamage` (`self.GetOwner`) (delegate `OnTakeAnyDamage_Event`)))

(event `OnTakeAnyDamage_Event`
  (params (DamagedActor :type "Actor Object Reference") (Damage :type "Float (single-precision)") (DamageType :type "DamageType Object Reference") (InstigatedBy :type "Controller Object Reference") (DamageCauser :type "Actor Object Reference"))
  (`self.Remove Health` Damage))

(fn `Give Health`
  (params (`Heal Amount` :type "Float (double-precision)"))
  (set `self.Health` (`KismetMathLibrary.FClamp` (+ `Heal Amount` (`self.Health`)) 0.0 (`self.Max Health`)))
  (message `/Game/Blueprints/BI_Coms.UpdateVisuals` (`self.GetOwner`) (`self.Health`) (<= (`self.Health`) 0.0)))

(fn `Remove Health`
  (params (Damage :type "Float (double-precision)"))
  (set `self.Health` (`KismetMathLibrary.FClamp` (- (`self.Health`) Damage) 0.0 (`self.Max Health`)))
  (message `/Game/Blueprints/BI_Coms.UpdateVisuals` (`self.GetOwner`) (`self.Health`) (<= (`self.Health`) 0.0)))