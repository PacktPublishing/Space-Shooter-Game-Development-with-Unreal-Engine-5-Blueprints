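; Parent enemy Blueprint that awards points and explodes when killed or when it collides with a body.
; UpdateVisuals with Dead set sends Points to the player pawn, then Death spawns an explosion emitter and destroys the actor.
; Overlap with a "Body"-tagged component sends Points to that actor, applies collision damage and calls Death.
; A helper function, not called here, smoothly rotates the enemy toward the player's pawn.
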(event `self.ReceiveBeginPlay`)

(event `/Game/Blueprints/BI_Coms.UpdateVisuals`
  (params (Hp :type "Float (double-precision)") (Dead :type Boolean))
  (if Dead
    (message `/Game/Blueprints/BI_Coms.Points Update` (`GameplayStatics.GetPlayerPawn` 0) (`self.Points`))
    (`self.Death`)))

(event `self.EnemyBody.OnComponentBeginOverlap`
  (params (OverlappedComponent :type "PrimitiveComponent Object Reference") (OtherActor :type "Actor Object Reference") (OtherComp :type "PrimitiveComponent Object Reference") (OtherBodyIndex :type Integer) (bFromSweep :type Boolean) (SweepResult :type "HitResult Structure (by ref)"))
  (`/Engine/EditorBlueprintResources/StandardMacros.IsValid` OtherComp
    (:`Is Valid`
      (if (`ActorComponent.ComponentHasTag` OtherComp "Body")
        (message `/Game/Blueprints/BI_Coms.Points Update` OtherActor (`self.Points`))
        (`GameplayStatics.ApplyDamage` OtherActor (`self.Collision Damage`))
        (`self.Death`)))))

(fn `Death`
  (`GameplayStatics.SpawnEmitterAtLocation` "/Game/Particles/P_Explosion.P_Explosion" (`self.K2_GetActorLocation`) (struct) (5.0 5.0 5.0))
  (`self.K2_DestroyActor`))

(fn `Update Rotation Towards player`
  (`/Engine/EditorBlueprintResources/StandardMacros.IsValid` (`Controller.K2_GetPawn` (`GameplayStatics.GetPlayerController` 0))
    (:`Is Valid`
      (`self.K2_SetActorRotation` (`KismetMathLibrary.RInterpTo` (`self.K2_GetActorRotation`) (`KismetMathLibrary.FindLookAtRotation` (`self.K2_GetActorLocation`) (`self.K2_GetActorLocation` (`Controller.K2_GetPawn` (`GameplayStatics.GetPlayerController` 0)))) (`GameplayStatics.GetWorldDeltaSeconds`) 10.0)))))

(fn `UserConstructionScript`)